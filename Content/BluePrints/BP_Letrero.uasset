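; BP_Letrero is a sign actor that displays the current level number (Nivel) as rendered text.
; On BeginPlay it finds all Teleport actors and writes the first one's Nivel to TextRender only; the matching TextRender1 node is unconnected.
; The CambioDeNivel and ResetNivel events are identical, refreshing both text components from that BeginPlay lookup's first Teleport.
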(event Custom|CambioDeNivel
  (Rendering|Components|TextRender|SetText (Variables|Default|GetTextRender) (Utilities|Text|ToText(Integer) (Variables|/Game/BluePrints/Teleport.Teleport_C|GetNivel (Utilities|Array|Get(acopy) (stale EventBeginPlay _outactors)))))
  (Rendering|Components|TextRender|SetText (Variables|Default|GetTextRender1) (Utilities|Text|ToText(Integer) (Variables|/Game/BluePrints/Teleport.Teleport_C|GetNivel (Utilities|Array|Get(acopy) (stale EventBeginPlay _outactors))))))

(event Custom|ResetNivel
  (Rendering|Components|TextRender|SetText (Variables|Default|GetTextRender) (Utilities|Text|ToText(Integer) (Variables|/Game/BluePrints/Teleport.Teleport_C|GetNivel (Utilities|Array|Get(acopy) (stale EventBeginPlay _outactors)))))
  (Rendering|Components|TextRender|SetText (Variables|Default|GetTextRender1) (Utilities|Text|ToText(Integer) (Variables|/Game/BluePrints/Teleport.Teleport_C|GetNivel (Utilities|Array|Get(acopy) (stale EventBeginPlay _outactors))))))

(event EventBeginPlay
  (bind _outactors (Actor|GetAllActorsOfClass "/Game/BluePrints/Teleport.Teleport_C"))
  (Rendering|Components|TextRender|SetText (Variables|Default|GetTextRender) (Utilities|Text|ToText(Integer) (Variables|/Game/BluePrints/Teleport.Teleport_C|GetNivel (Utilities|Array|Get(acopy) _outactors)))))

(event Collision|EventActorBeginOverlap
  (params (OtherActor :type Actor%20Object%20Reference)))

(event EventTick
  (params (DeltaSeconds :type Float%20%28single-precision%29)))

(fn ConstructionScript)