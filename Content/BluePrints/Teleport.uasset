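; Teleport trigger for a looping hallway with anomalies and a level counter.
; When BP_ThirdPersonCharacter overlaps the box, it moves the character to the arrow, keeping its rotation, and resets BP_Spline.
; TieneAnomalia decides whether Nivel resets to zero or increments, updating the BP_Letrero found at BeginPlay to match.
; It then calls Anomalias on BP_Pasillo, using the first instance found of each external actor.
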(event OnComponentBeginOverlap(Box)
  (params (OverlappedComponent :type Primitive%20Component%20Object%20Reference) (OtherActor :type Actor%20Object%20Reference) (OtherComp :type Primitive%20Component%20Object%20Reference) (OtherBodyIndex :type Integer) (bFromSweep :type Boolean) (SweepResult :type Hit%20Result%20Structure%20%28by%20ref%29))
  ;[0.1527 1 0.705] Spline
  (bind _asbp_third_person_character (Utilities|Casting|CastToBP_ThirdPersonCharacter OtherActor))
  (Transformation|SetActorLocationAndRotation _asbp_third_person_character (Transformation|GetWorldLocation (Variables|Default|GetArrow)) (Transformation|GetWorldRotation (Variables|/Script/Engine.Actor|GetRootComponent _asbp_third_person_character)))
  (bind _outactors (Actor|GetAllActorsOfClass "/Game/IA/AI_Characters/Spline/BP_Spline.BP_Spline_C"))
  (Default|ResetSpline (Utilities|Array|Get(acopy) _outactors))
  (if (Variables|Default|GetTieneAnomalia)
    (Development|PrintString "Reset")
    (bind _output_get (Variables|Default|SetNivel 0))
    (Development|PrintString (Utilities|String|ToString(Integer) _output_get))
    (Default|ResetNivel (Utilities|Array|Get(acopy) (stale EventBeginPlay _outactors)))
    (else
      (Development|PrintString "NextL")
      (bind _output_get_2 (Variables|Default|SetNivel (+ (Variables|Default|GetNivel) 1)))
      (Development|PrintString (Utilities|String|ToString(Integer) _output_get_2))
      (Default|CambioDeNivel (Utilities|Array|Get(acopy) (stale EventBeginPlay _outactors)))))
  (bind _outactors_2 (Actor|GetAllActorsOfClass "/Game/BluePrints/BP_Pasillo.BP_Pasillo_C"))
  (Default|Anomalias (Utilities|Array|Get(acopy) _outactors_2)))

(event EventBeginPlay
  (bind _outactors (Actor|GetAllActorsOfClass "/Game/BluePrints/BP_Letrero.BP_Letrero_C")))

(event Collision|EventActorBeginOverlap
  (params (OtherActor :type Actor%20Object%20Reference)))

(event EventTick
  (params (DeltaSeconds :type Float%20%28single-precision%29)))

(fn ConstructionScript)