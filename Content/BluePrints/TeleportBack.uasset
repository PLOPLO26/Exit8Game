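; Turn-back teleport trigger for a looping hallway anomaly game, where its box overlap scores the choice against the Teleport actor's TieneAnomalia flag.
; An anomaly raises Nivel, updates BP_Letrero, teleports BP_Anime to DestinationAnomalia, calls LookBack and resets BP_Spline; otherwise Nivel resets and BP_Anime moves to Destination.
; Both branches call BP_Pasillo's Anomalias, and level changes precede the BP_Anime cast, so any overlapping actor triggers them.
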(event OnComponentBeginOverlap(Box)
  (params (OverlappedComponent :type Primitive%20Component%20Object%20Reference) (OtherActor :type Actor%20Object%20Reference) (OtherComp :type Primitive%20Component%20Object%20Reference) (OtherBodyIndex :type Integer) (bFromSweep :type Boolean) (SweepResult :type Hit%20Result%20Structure%20%28by%20ref%29))
  (bind _destinationanomalia (Variables|Default|GetDestinationAnomalia))
  ;[0.1527 1 0.705] Spline
  (if (Variables|/Game/BluePrints/Teleport.Teleport_C|GetTieneAnomalia (Utilities|Array|Get(acopy) (stale EventBeginPlay _outactors)))
    (Development|PrintString "NextL")
    (bind _output_get (Variables|/Game/BluePrints/Teleport.Teleport_C|SetNivel (Utilities|Array|Get(acopy) (stale EventBeginPlay _outactors)) (+ (Variables|/Game/BluePrints/Teleport.Teleport_C|GetNivel (Utilities|Array|Get(acopy) (stale EventBeginPlay _outactors))) 1)))
    (Development|PrintString (Utilities|String|ToString(Integer) _output_get))
    (Default|CambioDeNivel (Utilities|Array|Get(acopy) (stale EventBeginPlay _outactors_3)))
    (bind _outactors (Actor|GetAllActorsOfClass "/Game/BluePrints/BP_Pasillo.BP_Pasillo_C"))
    (Default|Anomalias (Utilities|Array|Get(acopy) _outactors))
    (bind _asbp_anime (Utilities|Casting|CastToBP_Anime OtherActor))
    (Transformation|SetActorLocationAndRotation _asbp_anime (Transformation|GetWorldLocation _destinationanomalia) (Transformation|GetWorldRotation _destinationanomalia))
    (Default|LookBack (Utilities|Array|Get(acopy) (stale EventBeginPlay _outactors_4)))
    (bind _outactors_2 (Actor|GetAllActorsOfClass "/Game/IA/AI_Characters/Spline/BP_Spline.BP_Spline_C"))
    (Default|ResetSpline (Utilities|Array|Get(acopy) _outactors_2))
    (else
      (Development|PrintString "Reset")
      (bind _output_get_2 (Variables|/Game/BluePrints/Teleport.Teleport_C|SetNivel (Utilities|Array|Get(acopy) (stale EventBeginPlay _outactors)) 0))
      (Development|PrintString (Utilities|String|ToString(Integer) _output_get_2))
      (Default|ResetNivel (Utilities|Array|Get(acopy) (stale EventBeginPlay _outactors_3)))
      (bind _asbp_anime_2 (Utilities|Casting|CastToBP_Anime OtherActor))
      (Transformation|SetActorLocationAndRotation _asbp_anime_2 (Transformation|GetWorldLocation (Variables|Default|GetDestination)) (Transformation|GetWorldRotation (Variables|/Script/Engine.Actor|GetRootComponent _asbp_anime_2)))
      (bind _outactors_3 (Actor|GetAllActorsOfClass "/Game/BluePrints/BP_Pasillo.BP_Pasillo_C"))
      (Default|Anomalias (Utilities|Array|Get(acopy) _outactors_3)))))

(event EventBeginPlay
  (bind _outactors (Actor|GetAllActorsOfClass "/Game/BluePrints/Teleport.Teleport_C"))
  (bind _outactors_2 (Actor|GetAllActorsOfClass "/Game/ThirdPerson/Blueprints/BP_ThirdPersonCharacter.BP_ThirdPersonCharacter_C"))
  (bind _outactors_3 (Actor|GetAllActorsOfClass "/Game/BluePrints/BP_Letrero.BP_Letrero_C"))
  (bind _outactors_4 (Actor|GetAllActorsOfClass "/Game/Characters/anim2/BP_Anime.BP_Anime_C")))

(event Collision|EventActorBeginOverlap
  (params (OtherActor :type Actor%20Object%20Reference)))

(event EventTick
  (params (DeltaSeconds :type Float%20%28single-precision%29)))

(fn ConstructionScript)