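; BP_Pasillo is a hallway controller that randomly decides whether an anomaly appears on a painting (BP_Cuadro).
; On BeginPlay it looks up the BP_Cuadro and Teleport actors and uses the first of each.
; Anomalias picks between normal and anomaly states, updating the painting, the teleporter's TieneAnomalia flag and A1, with debug prints.
; ResetAnomali resets the painting only when A1 is false.
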(event Custom|Anomalias
  (switch int (Math|Random|RandomIntegerinRange 0 1)
    (:0
      (Development|PrintString "Default")
      (Default|ResetCuadro (Utilities|Array|Get(acopy) (stale EventBeginPlay _outactors)))
      (Variables|/Game/BluePrints/Teleport.Teleport_C|SetTieneAnomalia (Utilities|Array|Get(acopy) (stale EventBeginPlay _outactors_2)) false)
      (Variables|Default|SetA1 false))
    (:1
      (Development|PrintString "A1")
      (Variables|/Game/BluePrints/Teleport.Teleport_C|SetTieneAnomalia (Utilities|Array|Get(acopy) (stale EventBeginPlay _outactors_2)) true)
      (Default|Anomalia1 (Utilities|Array|Get(acopy) (stale EventBeginPlay _outactors)))
      (Variables|Default|SetA1 true))))

(event Custom|ResetAnomali
  (if (not (Variables|Default|GetA1))
    (Default|ResetCuadro (Utilities|Array|Get(acopy) (stale EventBeginPlay _outactors)))))

(event EventBeginPlay
  (bind _outactors (Actor|GetAllActorsOfClass "/Game/BluePrints/BP_Cuadro.BP_Cuadro_C"))
  (bind _outactors_2 (Actor|GetAllActorsOfClass "/Game/BluePrints/Teleport.Teleport_C")))

(fn ConstructionScript)